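; Railway carriage actor that can be placed along the track and opens or closes sliding doors on either side.
; NextTrolley moves the root to a given location using CarriageRotation and offsets two door meshes, mirrored on X.
; OpenDoors plays or reverses a timeline that lerps the chosen side's door and window components outward and apart in relative space.
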(event `Next Trolley`
  (params (`Carriage Location` :type "Vector Structure") (`Carriage Rotation` :type "Rotator Structure") (`Door X` :type "Float (double-precision)") (`Door Y` :type "Float (double-precision)"))
  (`SceneComponent.K2_SetWorldLocationAndRotation` (`self.DefaultSceneRoot`) `Carriage Location` (`KismetMathLibrary.MakeRotator` `Carriage Rotation_Roll` `Carriage Rotation_Pitch` (+ `Carriage Rotation_Yaw` 0.0)) false false)
  (`SceneComponent.K2_SetRelativeLocation` (`self.Train_26_Door`) (`KismetMathLibrary.MakeVector` `Door X` `Door Y`) false false)
  (`SceneComponent.K2_SetRelativeLocation` (`self.Train_26_Door_2`) (`KismetMathLibrary.MakeVector` (* `Door X` -1.0) `Door Y`) false false))

(event `Open Doors`
  (params (Open :type Boolean) (LeftSide :type Boolean))
  (if Open
    (bind (_direction _door_animation) (`Timeline|Door Animation` :!label _label)
      (:`Update`
        (if LeftSide
          (`SceneComponent.K2_SetRelativeLocation` (`self.Train_26_Door_window_4`) (`KismetMathLibrary.VLerp` (0.0 2.171588 51.987212) (-60.0 30.0 51.987212) _door_animation) false false)
          (`SceneComponent.K2_SetRelativeLocation` (`self.Train_26_Door_4`) (`KismetMathLibrary.VLerp` (0.0 2.171588 51.987212) (-60.0 30.0 51.987212) _door_animation) false false)
          (`SceneComponent.K2_SetRelativeLocation` (`self.Train_26_Door_2`) (`KismetMathLibrary.VLerp` (0.0 2.171588 51.987212) (-60.0 30.0 51.987212) _door_animation) false false)
          (`SceneComponent.K2_SetRelativeLocation` (`self.Train_26_Door_3`) (`KismetMathLibrary.VLerp` (0.0 2.171588 51.987212) (60.0 30.0 51.987212) _door_animation) false false)
          (`SceneComponent.K2_SetRelativeLocation` (`self.Train_26_Door`) (`KismetMathLibrary.VLerp` (0.0 2.171588 51.987212) (60.0 30.0 51.987212) _door_animation) false false)
          (`SceneComponent.K2_SetRelativeLocation` (`self.Train_26_Door_window_3`) (`KismetMathLibrary.VLerp` (0.0 2.171588 51.987212) (60.0 30.0 51.987212) _door_animation) false false)
          (else
            (`SceneComponent.K2_SetRelativeLocation` (`self.Train_26_Door_window_`) (`KismetMathLibrary.VLerp` (0.0 2.171588 51.987212) (-60.0 -30.0 51.987212) _door_animation) false false)
            (`SceneComponent.K2_SetRelativeLocation` (`self.Door_12`) (`KismetMathLibrary.VLerp` (0.0 2.171588 51.987212) (-60.0 -30.0 51.987212) _door_animation) false false)
            (`SceneComponent.K2_SetRelativeLocation` (`self.Door_9`) (`KismetMathLibrary.VLerp` (0.0 2.171588 51.987212) (-60.0 -30.0 51.987212) _door_animation) false false)
            (`SceneComponent.K2_SetRelativeLocation` (`self.Train_26_Door_window_2`) (`KismetMathLibrary.VLerp` (0.0 2.171588 51.987212) (60.0 -30.0 51.987212) _door_animation) false false)
            (`SceneComponent.K2_SetRelativeLocation` (`self.Door_11`) (`KismetMathLibrary.VLerp` (0.0 2.171588 51.987212) (60.0 -30.0 51.987212) _door_animation) false false)
            (`SceneComponent.K2_SetRelativeLocation` (`self.Door_10`) (`KismetMathLibrary.VLerp` (0.0 2.171588 51.987212) (60.0 -30.0 51.987212) _door_animation) false false)))))
    (else
      (goto _label :!via `Reverse`))))

(fn `UserConstructionScript`)