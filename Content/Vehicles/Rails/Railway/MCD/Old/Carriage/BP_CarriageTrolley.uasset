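; BP_CarriageTrolley is a railway carriage trolley that follows a spline track and positions the carriage bodies attached to it.
; CarriageTrolleyMove offsets the given distance by trolley number and a calibration value, then MoveAlong places the root on the spline with a yaw correction.
; It then sends its location, a look-at rotation toward NextTrolley and door values to valid regular and tail carriages.
; StopCarriage is an empty stub.
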(event `Stop Carriage`)

(event `Carriage Trolley Move`
  (params (Distance :type "Float (double-precision)") (DorX :type "Float (double-precision)") (DorY :type "Float (double-precision)"))
  (bind _holdable_carriage (`self.Holdable Carriage`))
  (bind _holdable_tail_carriage (`self.Holdable Tail Carriage`))
  (bind _returnvalue (`SceneComponent.K2_GetComponentLocation` (`self.DefaultSceneRoot`)))
  (bind _returnvalue_2 (`KismetMathLibrary.FindLookAtRotation` _returnvalue (`SceneComponent.K2_GetComponentLocation` (`/Game/Vehicles/Rails/Railway/MCD/Old/Carriage/BP_CarriageTrolley.DefaultSceneRoot` (`self.Next Trolley`)))))
  (`self.MoveAlong` (`/Game/MapBlueprints/Railways/Railways.Spline` (`self.ActivePath`)) (+ (* (`self.Trolley number`) -800) Distance (`self.Trolley cal`)))
  (if (`KismetSystemLibrary.IsValid` _holdable_carriage)
    (`/Game/Vehicles/Rails/Railway/MCD/Old/Carriage/BP_Carriage_Old.Next Trolley` _holdable_carriage _returnvalue _returnvalue_2 DorX DorY))
  (if (`KismetSystemLibrary.IsValid` _holdable_tail_carriage)
    (`/Game/Vehicles/Rails/Railway/MCD/Old/HeadCarriage/BP_TailCarriage_Old.Tail Carriage` _holdable_tail_carriage _returnvalue _returnvalue_2 DorX DorY)))

(fn `MoveAlong`
  (params (Path :type "SplineComponent Object Reference") (Distance :type "Float (double-precision)"))
  (bind (_returnvalue_roll _returnvalue_pitch _returnvalue_yaw) (`KismetMathLibrary.BreakRotator` (`SplineComponent.GetRotationAtDistanceAlongSpline` Path Distance "Local")))
  (`SceneComponent.K2_SetWorldLocationAndRotation` (`self.DefaultSceneRoot`) (+ (`SplineComponent.GetLocationAtDistanceAlongSpline` Path Distance "World") (0.0 0.0 0.0)) (`KismetMathLibrary.MakeRotator` _returnvalue_roll _returnvalue_pitch (+ (* _returnvalue_yaw 1.0) -90.0)) false false))

(fn `UserConstructionScript`)