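; Older tail carriage actor for the MCD train, placed from outside and animating its sliding doors on one side.
; The TailCarriage event sets the actor's location and rotation; its DoorX and DoorY inputs drive nothing live.
; OpenDoors plays or reverses a timeline that lerps the left or right door and window components outward between hardcoded relative positions.
; Some earlier direct transform nodes remain unconnected.
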(event `Tail Carriage`
  (params (`Carriage Location` :type "Vector Structure") (`Carriage Rotation` :type "Rotator Structure") (`Door X` :type "Float (double-precision)") (`Door Y` :type "Float (double-precision)"))
  (`self.K2_SetActorLocationAndRotation` `Carriage Location` `Carriage Rotation`))

(event `Open Doors`
  (params (Open :type Boolean) (`Left Side` :type Boolean))
  (if Open
    (bind (_direction `_новая_дорожка_0`) (`Timeline|Doors Animation` :!label _label)
      (:`Update`
        (if `Left Side`
          (`SceneComponent.K2_SetRelativeLocation` (`self.Head_Carriage_Door_head`) (`KismetMathLibrary.VLerp` (0.0 2.171588 51.987212) (-60.0 10.0 51.987212) `_новая_дорожка_0`) false false)
          (`SceneComponent.K2_SetRelativeLocation` (`self.Head_Carriage_Door_head_3`) (`KismetMathLibrary.VLerp` (0.0 2.171588 51.987212) (-60.0 10.0 51.987212) `_новая_дорожка_0`) false false)
          (`SceneComponent.K2_SetRelativeLocation` (`self.Door_7`) (`KismetMathLibrary.VLerp` (0.0 2.171588 51.987212) (60.0 10.0 51.987212) `_новая_дорожка_0`) false false)
          (`SceneComponent.K2_SetRelativeLocation` (`self.Head_Carriage_Door_window_head_2`) (`KismetMathLibrary.VLerp` (0.0 2.171588 51.987212) (60.0 10.0 51.987212) `_новая_дорожка_0`) false false)
          (else
            (`SceneComponent.K2_SetRelativeLocation` (`self.Head_Carriage_Door_head_2`) (`KismetMathLibrary.VLerp` (0.0 2.171588 51.987212) (-60.0 -10.0 51.987212) `_новая_дорожка_0`) false false)
            (`SceneComponent.K2_SetRelativeLocation` (`self.Head_Carriage_Door_head_4`) (`KismetMathLibrary.VLerp` (0.0 2.171588 51.987212) (-60.0 -10.0 51.987212) `_новая_дорожка_0`) false false)
            (`SceneComponent.K2_SetRelativeLocation` (`self.Door_8`) (`KismetMathLibrary.VLerp` (0.0 2.171588 51.987212) (60.0 -10.0 51.987212) `_новая_дорожка_0`) false false)
            (`SceneComponent.K2_SetRelativeLocation` (`self.Head_Carriage_Door_window_head_4`) (`KismetMathLibrary.VLerp` (0.0 2.171588 51.987212) (60.0 -10.0 51.987212) `_новая_дорожка_0`) false false)))))
    (else
      (goto _label :!via `Reverse`))))

(fn `UserConstructionScript`)