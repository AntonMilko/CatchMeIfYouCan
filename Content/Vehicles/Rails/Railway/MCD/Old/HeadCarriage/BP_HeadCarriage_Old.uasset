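; Legacy head carriage Blueprint for an MCD railway train, handling carriage placement and sliding passenger doors.
; HeadTrolley sets the root's world transform from a given location and stored rotation, and directly offsets one set of door meshes in mirrored X.
; OpenDoors plays or reverses a timeline that lerps door pairs outward and apart on the side selected by LeftSide.
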(event `HeadTrolley`
  (params (DoorX :type "Float (double-precision)") (DoorY :type "Float (double-precision)") (Location :type "Vector Structure") (Rotation :type "Rotator Structure"))
  (`SceneComponent.K2_SetWorldLocationAndRotation` (`self.DefaultSceneRoot`) Location (`KismetMathLibrary.MakeRotator` Rotation_Roll Rotation_Pitch (+ Rotation_Yaw 0.0)) false false)
  (`SceneComponent.K2_SetRelativeLocation` (`self.Head_Carriage_Door_head_2`) (`KismetMathLibrary.MakeVector` DoorX DoorY) false false)
  (`SceneComponent.K2_SetRelativeLocation` (`self.Head_Carriage_Door_head_4`) (`KismetMathLibrary.MakeVector` DoorX DoorY) false false)
  (`SceneComponent.K2_SetRelativeLocation` (`self.Head_Carriage_Door_head`) (`KismetMathLibrary.MakeVector` (* DoorX -1.0) DoorY) false false)
  (`SceneComponent.K2_SetRelativeLocation` (`self.Door_2`) (`KismetMathLibrary.MakeVector` (* DoorX -1.0) DoorY) false false))

(event `Open Doors`
  (params (Open :type Boolean) (`Left Side` :type Boolean))
  (if Open
    (bind (_direction _door_animation) (`Timeline|Door Animation` :!label _label)
      (:`Update`
        (if `Left Side`
          (`SceneComponent.K2_SetRelativeLocation` (`self.Head_Carriage_Door_head_2`) (`KismetMathLibrary.VLerp` (0.0 2.171588 51.987212) (60.0 10.0 51.987212) _door_animation) false false)
          (`SceneComponent.K2_SetRelativeLocation` (`self.Head_Carriage_Door_head_4`) (`KismetMathLibrary.VLerp` (0.0 2.171588 51.987212) (60.0 10.0 51.987212) _door_animation) false false)
          (`SceneComponent.K2_SetRelativeLocation` (`self.Door_2`) (`KismetMathLibrary.VLerp` (0.0 2.171588 51.987212) (-60.0 10.0 51.987212) _door_animation) false false)
          (`SceneComponent.K2_SetRelativeLocation` (`self.Head_Carriage_Door_head`) (`KismetMathLibrary.VLerp` (0.0 2.171588 51.987212) (-60.0 10.0 51.987212) _door_animation) false false)
          (else
            (`SceneComponent.K2_SetRelativeLocation` (`self.Head_Carriage_Door_head_3`) (`KismetMathLibrary.VLerp` (0.0 2.171588 51.987212) (60.0 -10.0 51.987212) _door_animation) false false)
            (`SceneComponent.K2_SetRelativeLocation` (`self.Head_Carriage_Door_window_head`) (`KismetMathLibrary.VLerp` (0.0 2.171588 51.987212) (60.0 -10.0 51.987212) _door_animation) false false)
            (`SceneComponent.K2_SetRelativeLocation` (`self.Door_7`) (`KismetMathLibrary.VLerp` (0.0 2.171588 51.987212) (-60.0 -10.0 51.987212) _door_animation) false false)
            (`SceneComponent.K2_SetRelativeLocation` (`self.Head_Carriage_Door_window_head_3`) (`KismetMathLibrary.VLerp` (0.0 2.171588 51.987212) (-60.0 -10.0 51.987212) _door_animation) false false)))))
    (else
      (goto _label :!via `Reverse`))))

(fn `UserConstructionScript`)