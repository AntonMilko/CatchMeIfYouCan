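; Lead trolley of a train that drives the head carriage and following carriages along a spline track.
; A timeline supplies speed and door offsets, and a short Delay loop advances the distance along the active path.
; Each step passes distance and doors to the carriage array and aims the head carriage at the next trolley.
; Stop reverses the timeline and stops the other carriage; at zero speed it waits, then restarts.
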(event `self.ReceiveBeginPlay`
  (bind _returnvalue (`SceneComponent.K2_GetComponentLocation` (`self.DefaultSceneRoot`)))
  (bind _spline (`/Game/MapBlueprints/Railways/Railways.Spline` (`self.ActivePath`)))
  (`TimelineComponent.SetPlayRate` (`self.Разгон поезда`) 15.0)
  (`KismetSystemLibrary.Delay` (`self.Tacting Mode`))
  (set `self.Travel` true :!label _label)
  (if (`self.Travel`)
    (bind (_direction _speed _door_y _door_x) (`Timeline|Разгон поезда` :!label _label_2)
      (:`Update`
        (set `self.Speed` _speed)
        (if (< (`self.Distance`) (`SplineComponent.GetSplineLength` _spline)) :!label _label_3
          (`self.MoveAlong_HeadCarriage` _spline (`self.Distance`))
          (`/Game/Vehicles/Rails/Railway/MCD/Old/Carriage/BP_CarriageTrolley.Carriage Trolley Move` (`self.Carriage Array`) (`self.Distance`) _door_x _door_y)
          (`/Game/Vehicles/Rails/Railway/MCD/Old/HeadCarriage/BP_HeadCarriage_Old.HeadTrolley` (`self.Holdable Head Carriage`) _door_x _door_y _returnvalue (`KismetMathLibrary.FindLookAtRotation` _returnvalue (`SceneComponent.K2_GetComponentLocation` (`/Game/Vehicles/Rails/Railway/MCD/Old/Carriage/BP_CarriageTrolley.DefaultSceneRoot` (`self.NextTrolley`)))))
          (set `self.Distance` (+ (`self.Distance`) (`self.Speed`)))
          (if (== (`self.Speed`) 0.0)
            (set `self.Travel` false)
            (`KismetSystemLibrary.Delay` (`self.StopTime`))
            (`self.Start`)
            (else
              (`KismetSystemLibrary.Delay` 0.001)
              (if (`self.Travel`)
                (goto _label_3)))))))))

(event `Start`
  (goto _label))

(event `Stop`
  (`/Game/Vehicles/Rails/Railway/MCD/Old/Carriage/BP_CarriageTrolley.Stop Carriage` (`self.Other Carriage`))
  (set `self.Travel` false)
  (goto _label_2 :!via `Reverse`))

(fn `MoveAlong_HeadCarriage`
  (params (Path :type "SplineComponent Object Reference") (Distance :type "Float (double-precision)"))
  (bind (_returnvalue_roll _returnvalue_pitch _returnvalue_yaw) (`KismetMathLibrary.BreakRotator` (`SplineComponent.GetRotationAtDistanceAlongSpline` Path Distance "Local")))
  (`SceneComponent.K2_SetWorldLocationAndRotation` (`self.DefaultSceneRoot`) (+ (`SplineComponent.GetLocationAtDistanceAlongSpline` Path Distance "World") (0.0 0.0 0.0)) (`KismetMathLibrary.MakeRotator` _returnvalue_roll _returnvalue_pitch (+ (* _returnvalue_yaw 1.0) -90.0)) false false))

(fn `UserConstructionScript`)