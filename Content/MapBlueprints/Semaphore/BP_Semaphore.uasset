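; BP_Semaphore is a traffic light actor that cycles endlessly through green, yellow, red and yellow from BeginPlay.
; A looping chain of Delays, timed by the GreenLight, YellowLight and RedLight variables, sets Signal to 0 for green, 1 for yellow or 2 for red.
; Each step swaps materials on the three lamp cylinders, giving the previous lamp NewMaterial and the active one its own material.
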(event `self.ReceiveBeginPlay`
  (`KismetSystemLibrary.Delay` (`self.GreenLight`) :!label _label)
  (set `self.Signal` 1)
  (`PrimitiveComponent.SetMaterial` (`self.Semaphore_Цилиндр_003`) 0 "/Game/MapBlueprints/Semaphore/NewMaterial.NewMaterial")
  (`PrimitiveComponent.SetMaterial` (`self.Semaphore_Цилиндр_002`) 0 "/Game/MapBlueprints/Semaphore/Материал_003.Материал_003")
  (`KismetSystemLibrary.Delay` (`self.YellowLight`))
  (set `self.Signal` 2)
  (`PrimitiveComponent.SetMaterial` (`self.Semaphore_Цилиндр_002`) 0 "/Game/MapBlueprints/Semaphore/NewMaterial.NewMaterial")
  (`PrimitiveComponent.SetMaterial` (`self.Semaphore_Цилиндр_001`) 0 "/Game/MapBlueprints/Semaphore/Материал_002.Материал_002")
  (`KismetSystemLibrary.Delay` (`self.RedLight`))
  (set `self.Signal` 1)
  (`PrimitiveComponent.SetMaterial` (`self.Semaphore_Цилиндр_001`) 0 "/Game/MapBlueprints/Semaphore/NewMaterial.NewMaterial")
  (`PrimitiveComponent.SetMaterial` (`self.Semaphore_Цилиндр_002`) 0 "/Game/MapBlueprints/Semaphore/Материал_003.Материал_003")
  (`KismetSystemLibrary.Delay` (`self.YellowLight`))
  (set `self.Signal` 0)
  (`PrimitiveComponent.SetMaterial` (`self.Semaphore_Цилиндр_002`) 0 "/Game/MapBlueprints/Semaphore/NewMaterial.NewMaterial")
  (`PrimitiveComponent.SetMaterial` (`self.Semaphore_Цилиндр_003`) 0 "/Game/MapBlueprints/Semaphore/Материал_004.Материал_004")
  (goto _label))

(fn `UserConstructionScript`)